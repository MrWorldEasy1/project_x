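; BP_Peephole is an interactable door peephole that lets the player look through it by switching the camera view.
; Interaction toggles watching: it blends the view target to the peephole actor holding the Eye component, or back to the player.
; While watching, it disables movement and controller-driven rotation, restoring both on exit.
; A Blink widget animation, timed with short delays, accompanies each camera blend.
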(event `self.ReceiveBeginPlay`
  (`parent.ReceiveBeginPlay`))

(event `/Game/ProjectX/Blueprints/InteractionSystem/BPI_Interact.Interaction`
  (params (Instigator :type "/Game/ProjectX/Character/Blueprints/Protagonist_Character Object Reference"))
  (bind _widget (`self.Widget`))
  (bind _firstpersoncamera (`/Game/ProjectX/Character/Blueprints/Protagonist_Character.FirstPersonCamera` Instigator))
  (bind _widget_2 (`self.Widget`))
  (if (`self.IsWatch`)
    (`PlayerController.SetViewTargetWithBlend` (`GameplayStatics.GetPlayerController` 0) (`ActorComponent.GetOwner` _firstpersoncamera) 0.5 "VTBlend_Linear" 0.0 false)
    (`UserWidget.PlayAnimation` _widget (`/Game/ProjectX/Blueprints/InteractionSystem/Blink_Widget.Blink` _widget) 0.0 1 "Forward" 0.75)
    (`KismetSystemLibrary.Delay` 0.45)
    (`Widget.RemoveFromParent` (`self.Widget`))
    (set `CameraComponent.bUsePawnControlRotation` true _firstpersoncamera)
    (set `Pawn.bUseControllerRotationYaw` true Instigator)
    (`CharacterMovementComponent.SetMovementMode` (`Character.CharacterMovement` Instigator) "MOVE_Walking" 0)
    (set `self.IsWatch` false)
    (else
      (bind _returnvalue (`|CreateWidget` "/Game/ProjectX/Blueprints/InteractionSystem/Blink_Widget.Blink_Widget_C"))
      (bind _output_get (set `self.Widget` _returnvalue))
      (`UserWidget.AddToViewport` _output_get 0)
      (`CharacterMovementComponent.DisableMovement` (`Character.CharacterMovement` Instigator))
      (set `CameraComponent.bUsePawnControlRotation` false (`/Game/ProjectX/Character/Blueprints/Protagonist_Character.FirstPersonCamera` Instigator))
      (set `Pawn.bUseControllerRotationYaw` false Instigator)
      (set `self.IsWatch` true)
      (`PlayerController.SetViewTargetWithBlend` (`GameplayStatics.GetPlayerController` 0) (`ActorComponent.GetOwner` (`self.Eye`)) 0.6 "VTBlend_Linear" 0.0 false)
      (`KismetSystemLibrary.Delay` 0.35)
      (`UserWidget.PlayAnimation` _widget_2 (`/Game/ProjectX/Blueprints/InteractionSystem/Blink_Widget.Blink` _widget_2) 0.0 1 "Forward" 0.75))))

(fn `UserConstructionScript`
  (`parent.UserConstructionScript`))