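; BP_OutsideDoor is an outside door actor with an InteractLocation overlap trigger for the protagonist.
; Begin and end overlap events cast to Protagonist_Character and only print "In" or "Out" as debug feedback.
; Disconnected nodes hold an unused camera blend between the door's Camera and the player's first-person camera, toggling pawn control rotation.
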(event `self.InteractLocation.OnComponentBeginOverlap`
  (params (OverlappedComponent :type "PrimitiveComponent Object Reference") (OtherActor :type "Actor Object Reference") (OtherComp :type "PrimitiveComponent Object Reference") (OtherBodyIndex :type Integer) (bFromSweep :type Boolean) (SweepResult :type "HitResult Structure (by ref)"))
  (bind _asprotagonist_character (cast `/Game/ProjectX/Character/Blueprints/Protagonist_Character` OtherActor))
  (`KismetSystemLibrary.PrintString` "In"))

(event `self.InteractLocation.OnComponentEndOverlap`
  (params (OverlappedComponent :type "PrimitiveComponent Object Reference") (OtherActor :type "Actor Object Reference") (OtherComp :type "PrimitiveComponent Object Reference") (OtherBodyIndex :type Integer))
  (bind _asprotagonist_character (cast `/Game/ProjectX/Character/Blueprints/Protagonist_Character` OtherActor))
  (`KismetSystemLibrary.PrintString` "Out"))

(event `InputAction|Interaction`
  (params (Key :type "Key Structure")))

(fn `UserConstructionScript`)