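; BP_Switch_Double is a double switch prop with two button meshes that can each appear lit or unlit.
; The construction script reads the Light1 and Light2 flags and sets the Emissive_Power material parameter on the matching button to glowing or off.
; The file shows no runtime logic, only this construction-time setup of each button's look.
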(fn `UserConstructionScript`
  (bind _sm_switch_button (`self.SM_Switch_Button`))
  (bind _sm_switch_button2 (`self.SM_Switch_Button2`))
  (`|ExecutionSequence`
    (:`then_0`
      (if (`self.Light_1`)
        (`MeshComponent.SetScalarParameterValueOnMaterials` _sm_switch_button "Emissive_Power" 5.0)
        (else
          (`MeshComponent.SetScalarParameterValueOnMaterials` _sm_switch_button "Emissive_Power" 0.0))))
    (:`then_1`
      (if (`self.Light_2`)
        (`MeshComponent.SetScalarParameterValueOnMaterials` _sm_switch_button2 "Emissive_Power" 5.0)
        (else
          (`MeshComponent.SetScalarParameterValueOnMaterials` _sm_switch_button2 "Emissive_Power" 0.0))))))